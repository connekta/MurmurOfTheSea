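; Spawner actor that populates a box volume with Fish_01 child actors on BeginPlay, up to NumberOfSharksToSpawn.
; A counter-driven loop line-traces downward from random XY points in Box at BoxRoof height, with debug drawing.
; Each fish is added as a child actor component, placed above the impact point on a hit or at the trace end otherwise.
; The construction script is empty, and older SpawnActor and construction-time versions remain disconnected.
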(event EventBeginPlay
  (bind _box (Variables|Default|GetBox))
  (bind _boxroof (Variables|Default|GetBoxRoof))
  (bind _returnvalue (Transformation|GetWorldLocation _boxroof))
  (bind _returnvalue_2 (Components|Box|GetScaledBoxExtent _box))
  (bind _returnvalue_3 (Transformation|GetWorldLocation _box))
  (bind _returnvalue_4 (Math|Random|RandomPointinBoundingBox _returnvalue_3 _returnvalue_2))
  (bind _returnvalue_5 (Math|Vector|MakeVector (.x _returnvalue_4) (.y _returnvalue_4) (.z _returnvalue)))
  (if (not (>= (Variables|Default|GetSpawnedSharks) (Variables|Default|GetNumberOfSharksToSpawn))) :!label _label
    (Math|Integer|IncrementInt (Variables|Default|GetSpawnedSharks)
      (:%20%20
        (bind _outhit (Collision|LineTraceForObjects _returnvalue_5 (- _returnvalue_5 "0, 0,1000.000000") (Utilities|Array|MakeArray "ObjectTypeQuery1" "ObjectTypeQuery2") false 0 "ForDuration"))
        (if (.bblockinghit _outhit)
          (bind _returnvalue_6 (AddComponent|AddChildActorComponent false))
          (ChildActorComponent|SetChildActorClass _returnvalue_6 "/Game/Blueprints/Fish_01.Fish_01_C")
          (Transformation|SetWorldLocationAndRotation _returnvalue_6 (+ (.impactpoint _outhit) "0, 0,250.000000") "0, 0, 0" false false)
          (goto _label)
          (else
            (bind _returnvalue_7 (AddComponent|AddChildActorComponent false))
            (ChildActorComponent|SetChildActorClass _returnvalue_7 "/Game/Blueprints/Fish_01.Fish_01_C")
            (Transformation|SetWorldLocationAndRotation _returnvalue_7 (.traceend _outhit) "0, 0, 0" false false)
            (goto _label)))))))

(fn ConstructionScript)
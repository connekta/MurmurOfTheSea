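; Wandering fish actor that picks random underwater headings and reacts when the player character or rowboat comes close.
; Box traces test random points ahead at clamped depth, and the looping Turn timeline rotates the capsule toward clear ones.
; Repeated blockage or player overlap halts turning, pulses a Turn180 flag and picks a new heading after a delay.
; A periodic distance check destroys fish far from the player; the Swim movement timeline is disconnected.
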(event OnComponentBeginOverlap(PlayerDetection)
  (params (OverlappedComponent :type Primitive%20Component%20Object%20Reference) (OtherActor :type Actor%20Object%20Reference) (OtherComp :type Primitive%20Component%20Object%20Reference) (OtherBodyIndex :type Integer) (bFromSweep :type Boolean) (SweepResult :type Hit%20Result%20Structure%20%28by%20ref%29))
  (bind _returnvalue (Utilities|GetClass OtherActor))
  ;[1 1 1] Turn If close To Player
  (if (or (== _returnvalue "/Game/ThirdPersonBP/Blueprints/ThirdPersonCharacter.ThirdPersonCharacter_C") (== _returnvalue "/Game/CartoonWaterShader/Meshes/RowBoat/BP_Rowboat.BP_Rowboat_C"))
    (Utilities|FlowControl|DoOnce false
      (:Completed
        (CallFunction|StopRotating)
        (Variables|Default|SetTurn180 true)
        (Utilities|FlowControl|Delay 0.2)
        (Variables|Default|SetTurn180 false)))))

(event OnComponentEndOverlap(PlayerDetection)
  (params (OverlappedComponent :type Primitive%20Component%20Object%20Reference) (OtherActor :type Actor%20Object%20Reference) (OtherComp :type Primitive%20Component%20Object%20Reference) (OtherBodyIndex :type Integer))
  (bind _returnvalue (Utilities|GetClass OtherActor))
  ;[1 1 1] Turn If close To Player
  (if (or (== _returnvalue "/Game/ThirdPersonBP/Blueprints/ThirdPersonCharacter.ThirdPersonCharacter_C") (== _returnvalue "/Game/CartoonWaterShader/Meshes/RowBoat/BP_Rowboat.BP_Rowboat_C"))
    (Utilities|FlowControl|DoOnce false) ; enters at Reset
  ))

(event Custom|TurnAround
  (bind _returnvalue (Math|Random|RandomFloatinRange -1.8e+02 1.8e+02))
  (bind _returnvalue_2 (Math|Random|RandomFloatinRange -1.8e+02 1.8e+02))
  (bind _returnvalue_3 (Math|Random|RandomFloatinRange -25.0 25.0))
  (bind _returnvalue_4 (Math|Random|RandomFloatinRange -1.8e+02 1.8e+02))
  (bind _returnvalue_5 (Math|Random|RandomFloatinRange -1.8e+02 1.8e+02))
  (bind _returnvalue_6 (Math|Random|RandomFloatinRange -25.0 25.0))
  (bind _self self)
  (bind _self_2 self)
  (bind _returnvalue_7 (Transformation|GetActorLocation _self))
  (bind _returnvalue_8 (Transformation|GetActorForwardVector _self))
  (bind _returnvalue_9 (Transformation|GetActorLocation _self_2))
  (bind _returnvalue_10 (Transformation|GetActorForwardVector _self_2))
  (bind _returnvalue_11 (* _returnvalue_8 350))
  (bind _returnvalue_12 (* _returnvalue_10 -350))
  (bind _returnvalue_13 (+ _returnvalue_7 _returnvalue_11))
  (bind _returnvalue_14 (+ _returnvalue_9 _returnvalue_12))
  (bind _returnvalue_15 (+ _returnvalue_13 (Math|Vector|MakeVector _returnvalue _returnvalue_2 _returnvalue_3)))
  (bind _returnvalue_16 (+ _returnvalue_14 (Math|Vector|MakeVector _returnvalue_4 _returnvalue_5 _returnvalue_6)))
  (bind (_x _y _z) (Math|Vector|BreakVector _returnvalue_15))
  (bind (_x_2 _y_2 _z_2) (Math|Vector|BreakVector _returnvalue_16))
  (Variables|Default|SetTimesTried 0)
  (bind _outhit (Class|KismetSystemLibrary|BoxTraceSingleforObjects _returnvalue_7 (Variables|Default|GetTraceEnd) "25.000000,25.000000,25.000000" "0, 0, 0" (Utilities|Array|MakeArray "ObjectTypeQuery1" "ObjectTypeQuery2") false 0 "None" true :!label _label))
  (if (.bblockinghit _outhit)
    (bind _result (Math|Integer|IncrementInt (Variables|Default|GetTimesTried))
      (:%20%20
        (if (> _result 10)
          (Variables|Default|SetTimesTried 0)
          (Variables|Default|SetTraceEnd (Math|Vector|MakeVector _x_2 _y_2 (Math|Float|Clamp(Float) _z_2 -1e+03 -5e+01)))
          (CallFunction|StopRotating)
          (Variables|Default|SetTurn180 true)
          (Utilities|FlowControl|Delay 0.2)
          (Variables|Default|SetTurn180 false)
          (else
            (goto _label)))))
    (else
      (bind _newtrack_0 (Timeline|Turn PlayFromStart)
        (:Update
          (Transformation|SetWorldRotation (Variables|Collision|GetCapsuleComponent) (Math|Rotator|Lerp(Rotator) (Variables|Default|GetPrevRot) (Math|Rotator|FindLookatRotation (Variables|Default|GetPrevPos) (.traceend _outhit)) _newtrack_0 true) false false))
        (:Finished
          (Variables|Default|SetTraceEnd (Math|Vector|MakeVector _x _y (Math|Float|Clamp(Float) _z -1e+03 -5e+01)))
          (Variables|Default|SetTimesTried 0)
          (Variables|Default|SetPrevPos _returnvalue_7)
          (Variables|Default|SetPrevRot (Transformation|GetWorldRotation (Variables|Collision|GetCapsuleComponent)))
          (goto _label))))))

(event Custom|StopRotating
  (bind _returnvalue (Math|Random|RandomFloatinRange -1.8e+02 1.8e+02))
  (bind _returnvalue_2 (Math|Random|RandomFloatinRange -1.8e+02 1.8e+02))
  (bind _returnvalue_3 (Math|Random|RandomFloatinRange -25.0 25.0))
  (bind _returnvalue_4 (Math|Random|RandomFloatinRange -1.8e+02 1.8e+02))
  (bind _returnvalue_5 (Math|Random|RandomFloatinRange -1.8e+02 1.8e+02))
  (bind _returnvalue_6 (Math|Random|RandomFloatinRange -25.0 25.0))
  (bind _self self)
  (bind _self_2 self)
  (bind _returnvalue_7 (Transformation|GetActorLocation _self))
  (bind _returnvalue_8 (Transformation|GetActorForwardVector _self))
  (bind _returnvalue_9 (Transformation|GetActorLocation _self_2))
  (bind _returnvalue_10 (Transformation|GetActorForwardVector _self_2))
  (bind _returnvalue_11 (* _returnvalue_8 350))
  (bind _returnvalue_12 (* _returnvalue_10 -350))
  (bind _returnvalue_13 (+ _returnvalue_7 _returnvalue_11))
  (bind _returnvalue_14 (+ _returnvalue_9 _returnvalue_12))
  (bind _returnvalue_15 (+ _returnvalue_13 (Math|Vector|MakeVector _returnvalue _returnvalue_2 _returnvalue_3)))
  (bind _returnvalue_16 (+ _returnvalue_14 (Math|Vector|MakeVector _returnvalue_4 _returnvalue_5 _returnvalue_6)))
  (bind (_x _y _z) (Math|Vector|BreakVector _returnvalue_15))
  (bind (_x_2 _y_2 _z_2) (Math|Vector|BreakVector _returnvalue_16))
  (Utilities|FlowControl|Sequence
    (:then_0
      (bind _newtrack_0 (Timeline|Turn Stop)
        (:Update
          (Transformation|SetWorldRotation (Variables|Collision|GetCapsuleComponent) (Math|Rotator|Lerp(Rotator) (Variables|Default|GetPrevRot) (Math|Rotator|FindLookatRotation (Variables|Default|GetPrevPos) (.traceend (stale _outhit))) _newtrack_0 true) false false))
        (:Finished
          (Variables|Default|SetTraceEnd (Math|Vector|MakeVector _x _y (Math|Float|Clamp(Float) _z -1e+03 -5e+01)) :!label _label)
          (Variables|Default|SetTimesTried 0)
          (Variables|Default|SetPrevPos _returnvalue_7)
          (Variables|Default|SetPrevRot (Transformation|GetWorldRotation (Variables|Collision|GetCapsuleComponent)))
          (bind _outhit (Class|KismetSystemLibrary|BoxTraceSingleforObjects _returnvalue_7 (Variables|Default|GetTraceEnd) "25.000000,25.000000,25.000000" "0, 0, 0" (Utilities|Array|MakeArray "ObjectTypeQuery1" "ObjectTypeQuery2") false 0 "None" true :!label _label_2))
          (if (.bblockinghit _outhit)
            (bind _result (Math|Integer|IncrementInt (Variables|Default|GetTimesTried))
              (:%20%20
                (if (> _result 10)
                  (Variables|Default|SetTimesTried 0)
                  (Variables|Default|SetTraceEnd (Math|Vector|MakeVector _x_2 _y_2 (Math|Float|Clamp(Float) _z_2 -1e+03 -5e+01)))
                  (CallFunction|StopRotating)
                  (Variables|Default|SetTurn180 true)
                  (Utilities|FlowControl|Delay 0.2)
                  (Variables|Default|SetTurn180 false)
                  (else
                    (goto _label_2)))))
            (else
              (Timeline|Turn PlayFromStart))))))
    (:then_1
      (Utilities|FlowControl|Delay 2.0)
      (goto _label))))

(event EventBeginPlay
  (bind _returnvalue (Math|Random|RandomFloatinRange -1.8e+02 1.8e+02))
  (bind _returnvalue_2 (Math|Random|RandomFloatinRange -1.8e+02 1.8e+02))
  (bind _returnvalue_3 (Math|Random|RandomFloatinRange -25.0 25.0))
  (bind _returnvalue_4 (Math|Random|RandomFloatinRange -1.8e+02 1.8e+02))
  (bind _returnvalue_5 (Math|Random|RandomFloatinRange -1.8e+02 1.8e+02))
  (bind _returnvalue_6 (Math|Random|RandomFloatinRange -25.0 25.0))
  (bind _self self)
  (bind _self_2 self)
  (bind _returnvalue_7 (Transformation|GetActorLocation _self))
  (bind _returnvalue_8 (Transformation|GetActorForwardVector _self))
  (bind _returnvalue_9 (Transformation|GetActorLocation _self_2))
  (bind _returnvalue_10 (Transformation|GetActorForwardVector _self_2))
  (bind _returnvalue_11 (* _returnvalue_8 350))
  (bind _returnvalue_12 (* _returnvalue_10 -350))
  (bind _returnvalue_13 (+ _returnvalue_7 _returnvalue_11))
  (bind _returnvalue_14 (+ _returnvalue_9 _returnvalue_12))
  (bind _returnvalue_15 (+ _returnvalue_13 (Math|Vector|MakeVector _returnvalue _returnvalue_2 _returnvalue_3)))
  (bind _returnvalue_16 (+ _returnvalue_14 (Math|Vector|MakeVector _returnvalue_4 _returnvalue_5 _returnvalue_6)))
  (bind (_x _y _z) (Math|Vector|BreakVector _returnvalue_15))
  (bind (_x_2 _y_2 _z_2) (Math|Vector|BreakVector _returnvalue_16))
  (bind _asthird_person_character (Utilities|Casting|CastToThirdPersonCharacter (Game|GetPlayerCharacter 0))
    (:then
      (Variables|Default|SetPlayerRef _asthird_person_character))
    (:CastFailed
      _))
  (Utilities|FlowControl|Sequence
    (:then_0
      (Variables|Default|SetTraceEnd (Math|Vector|MakeVector _x _y (Math|Float|Clamp(Float) _z -1e+03 -5e+01)) :!label _label)
      (Variables|Default|SetTimesTried 0)
      (Variables|Default|SetPrevPos _returnvalue_7)
      (Variables|Default|SetPrevRot (Transformation|GetWorldRotation (Variables|Collision|GetCapsuleComponent)))
      (bind _outhit (Class|KismetSystemLibrary|BoxTraceSingleforObjects _returnvalue_7 (Variables|Default|GetTraceEnd) "25.000000,25.000000,25.000000" "0, 0, 0" (Utilities|Array|MakeArray "ObjectTypeQuery1" "ObjectTypeQuery2") false 0 "None" true :!label _label_2))
      (if (.bblockinghit _outhit)
        (bind _result (Math|Integer|IncrementInt (Variables|Default|GetTimesTried))
          (:%20%20
            (if (> _result 10)
              (Variables|Default|SetTimesTried 0)
              (Variables|Default|SetTraceEnd (Math|Vector|MakeVector _x_2 _y_2 (Math|Float|Clamp(Float) _z_2 -1e+03 -5e+01)))
              (CallFunction|StopRotating)
              (Variables|Default|SetTurn180 true)
              (Utilities|FlowControl|Delay 0.2)
              (Variables|Default|SetTurn180 false)
              (else
                (goto _label_2)))))
        (else
          (bind _newtrack_0 (Timeline|Turn PlayFromStart)
            (:Update
              (Transformation|SetWorldRotation (Variables|Collision|GetCapsuleComponent) (Math|Rotator|Lerp(Rotator) (Variables|Default|GetPrevRot) (Math|Rotator|FindLookatRotation (Variables|Default|GetPrevPos) (.traceend _outhit)) _newtrack_0 true) false false))
            (:Finished
              (goto _label))))))
    (:then_1
      (if (> (Transformation|GetDistanceTo (Variables|Default|GetPlayerRef)) 5e+03) :!label _label_3
        (Actor|DestroyActor)
        (Development|PrintString "Shark Destroyed By Manual Cullling")
        (else
          (Utilities|FlowControl|Delay 15.0)
          (goto _label_3))))))

(fn ConstructionScript)
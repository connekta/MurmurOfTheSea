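; Wind ribbon box actor that scatters wind ribbon particle effects through a box volume to visualize the level's wind.
; On BeginPlay a fast looping timer spawns a Wind_ribbon emitter at a random point within the Box component's bounds.
; Each emitter takes its rotation from the first WindDirectionalSource found, which is looked up again on every spawn.
; If no wind source exists, it prints a debug message instead.
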(event Custom|spawnribbon
  (bind _box (Variables|Default|GetBox))
  (bind (_origin _boxextent) (Collision|GetComponentBounds _box))
  (bind _outactors (Actor|GetAllActorsOfClass "/Script/Engine.WindDirectionalSource"))
  (Utilities|IsValid (Utilities|Array|Get(acopy) _outactors)
    (:Is%20Valid
      (Effects|SpawnEmitteratLocation "/Game/Assets/Materials/wind_ribbon.wind_ribbon" (Math|Random|RandomPointinBoundingBox _origin _boxextent) (Transformation|GetWorldRotation (Variables|/Script/Engine.WindDirectionalSource|GetComponent (Utilities|Array|Get(acopy) _outactors)))))
    (:Is%20Not%20Valid
      (Development|PrintString "NOT VLAID BOX"))))

(event EventBeginPlay
  ;[1 1 1] Comment
  (Utilities|Time|SetTimerbyEvent (delegate Custom|spawnribbon) 0.1 true))

(fn ConstructionScript)
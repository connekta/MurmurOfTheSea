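; Underwater air bubble actor that gives the third-person character a dry pocket inside the cartoon-water ocean.
; Capsule overlap toggles the player's underwater state and bubble reference, and shows a cable holder placed at the head socket.
; Camera-collider overlap disables or restores the ocean's underwater effect and toggles a post-process.
; Tick fades the dynamic bubble material's opacity and rim light with player distance.
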(event OnComponentBeginOverlap(StaticMeshComponent)
  (params (OverlappedComponent :type Primitive%20Component%20Object%20Reference) (OtherActor :type Actor%20Object%20Reference) (OtherComp :type Primitive%20Component%20Object%20Reference) (OtherBodyIndex :type Integer) (bFromSweep :type Boolean) (SweepResult :type Hit%20Result%20Structure%20%28by%20ref%29))
  (bind _cableholder (Variables|Default|GetCableHolder))
  (bind _playerref (Variables|Default|GetPlayerRef))
  (bind _playerref_2 (Variables|Default|GetPlayerRef))
  (if (== OtherComp (Variables|/Script/Engine.Character|GetCapsuleComponent _playerref))
    (Default|UnderWater _playerref_2 false)
    (Variables|/Game/ThirdPersonBP/Blueprints/ThirdPersonCharacter.ThirdPersonCharacter_C|SetInsideWaterBubble _playerref_2 true)
    (Variables|/Game/ThirdPersonBP/Blueprints/ThirdPersonCharacter.ThirdPersonCharacter_C|SetWaterBubbleRef _playerref_2 self)
    (Transformation|SetWorldLocation _cableholder (Transformation|GetSocketLocation (Variables|/Script/Engine.Character|GetMesh _playerref_2) "Head") false false)
    (Rendering|SetVisibility _cableholder true false)
    (elif (== OtherComp (Variables|/Game/ThirdPersonBP/Blueprints/ThirdPersonCharacter.ThirdPersonCharacter_C|GetCameraCol _playerref))
      (Default|CustomDisableUnderwater (Variables|Default|GetOceanRef))
      (Variables|/Script/Engine.PostProcessVolume|SetbEnabled (Variables|Default|GetConnectedPostProcess) true))))

(event OnComponentEndOverlap(StaticMeshComponent)
  (params (OverlappedComponent :type Primitive%20Component%20Object%20Reference) (OtherActor :type Actor%20Object%20Reference) (OtherComp :type Primitive%20Component%20Object%20Reference) (OtherBodyIndex :type Integer))
  (bind _playerref (Variables|Default|GetPlayerRef))
  (bind _playerref_2 (Variables|Default|GetPlayerRef))
  (if (== OtherComp (Variables|/Script/Engine.Character|GetCapsuleComponent _playerref_2))
    (Default|UnderWater _playerref true)
    (Variables|/Game/ThirdPersonBP/Blueprints/ThirdPersonCharacter.ThirdPersonCharacter_C|SetInsideWaterBubble _playerref false)
    (Variables|/Game/ThirdPersonBP/Blueprints/ThirdPersonCharacter.ThirdPersonCharacter_C|SetWaterBubbleRef _playerref 0)
    (Rendering|SetVisibility (Variables|Default|GetCableHolder) false false)
    (elif (== OtherComp (Variables|/Game/ThirdPersonBP/Blueprints/ThirdPersonCharacter.ThirdPersonCharacter_C|GetCameraCol _playerref_2))
      (Default|CustomEnableUnderwater (Variables|Default|GetOceanRef))
      (Variables|/Script/Engine.PostProcessVolume|SetbEnabled (Variables|Default|GetConnectedPostProcess) false))))

(event EventTick
  (params (DeltaSeconds :type Float%20%28single-precision%29))
  (bind _playerref (Variables|Default|GetPlayerRef))
  (bind _materialref (Variables|Default|GetMaterialRef))
  (bind _returnvalue (Transformation|GetDistanceTo _playerref))
  (bind _returnvalue_2 (Math|Float|MapRangeClamped _returnvalue 1.5e+03 4e+03 0.0 1.0))
  ;[1 1 1] CLEANUP THIS
  (Utilities|IsValid (Variables|Default|GetMaterialRef)
    (:Is%20Valid
      (Rendering|Material|SetScalarParameterValue _materialref "Opacity" (Math|Float|Lerp 0.7 0.1 _returnvalue_2) :!class /Script/Engine.MaterialInstanceDynamic)
      (Rendering|Material|SetScalarParameterValue _materialref "RimlightOpacity" (Math|Float|Lerp 1.0 0.1 _returnvalue_2) :!class /Script/Engine.MaterialInstanceDynamic))))

(event EventBeginPlay
  ;[1 1 1] EventBeginPlay
  (Utilities|FlowControl|Delay 0.2)
  (bind _asthird_person_character (Utilities|Casting|CastToThirdPersonCharacter (Game|GetPlayerCharacter 0)))
  (Variables|Default|SetPlayerRef _asthird_person_character)
  (bind _outactors (Actor|GetAllActorsOfClass "/Game/CartoonWaterShader/Blueprints/CartoonWaterBlueprints/BP_CartoonWater_Ocean.BP_CartoonWater_Ocean_C"))
  (Variables|Default|SetOceanRef (Utilities|Array|Get(acopy) _outactors))
  (bind _returnvalue (Rendering|Material|CreateDynamicMaterialInstance (Variables|Debug|GetStaticMeshComponent) 0 "/Game/CartoonWaterShader/Materials/Water/Waterfall/UnderWaterBubbleInside.UnderWaterBubbleInside" "None" :!class /Script/Engine.PrimitiveComponent))
  (Variables|Default|SetMaterialRef _returnvalue))

(fn ConstructionScript)
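; Energy_Ball is a floating object whose mesh bobs vertically in a continuous loop around its starting position.
; On BeginPlay it caches the mesh's world location, then the Bounce timeline adds its track value to Z and restarts itself through a custom event when finished.
; A Sphere overlap with a BP_Rowboat only prints a "Hello" debug string, with no pickup or gameplay effect.
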(event OnComponentBeginOverlap(Sphere)
  (params (OverlappedComponent :type Primitive%20Component%20Object%20Reference) (OtherActor :type Actor%20Object%20Reference) (OtherComp :type Primitive%20Component%20Object%20Reference) (OtherBodyIndex :type Integer) (bFromSweep :type Boolean) (SweepResult :type Hit%20Result%20Structure%20%28by%20ref%29))
  (if (== (Utilities|GetClass OtherActor) "/Game/CartoonWaterShader/Meshes/RowBoat/BP_Rowboat.BP_Rowboat_C")
    (Development|PrintString "Hello")))

(event Custom|startbounce
  (bind _start_location (Variables|Default|Getstart_location))
  (bind (_x _y _z) (Math|Vector|BreakVector _start_location))
  (bind _newtrack_0 (Timeline|bounce PlayFromStart)
    (:Update
      (Transformation|SetWorldLocation (Variables|Default|GetStaticMesh) (Math|Vector|MakeVector _x _y (+ _z _newtrack_0)) false false))
    (:Finished
      (CallFunction|Startbounce))))

(event EventBeginPlay
  (Variables|Default|Setstart_location (Transformation|GetWorldLocation (Variables|Default|GetStaticMesh)))
  (bind _newtrack_0 (Timeline|bounce PlayFromStart)
    (:Update
      (Transformation|SetWorldLocation (Variables|Default|GetStaticMesh) (Math|Vector|MakeVector (.X (Math|Vector|BreakVector (Variables|Default|Getstart_location))) (.Y (Math|Vector|BreakVector (Variables|Default|Getstart_location))) (+ (.Z (Math|Vector|BreakVector (Variables|Default|Getstart_location))) _newtrack_0)) false false))
    (:Finished
      (CallFunction|Startbounce))))

(fn ConstructionScript)